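; Ball actor that, once its buff is activated, changes the movement speed of XR characters that touch it.
; BuffActive swaps the ball's material, sets the actor's lifespan and flags the buff as active.
; A sphere overlap handler bound at BeginPlay checks that flag, then passes the BuffActive speed ratio to the overlapping BP_XRCharacter's MoveSpeedChange.
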(event `BuffActive`
  (params (SpeedRatio :type "Float (double-precision)") (LifeSpan :type "Float (double-precision)"))
  (`PrimitiveComponent.SetMaterial` (`self.ball`) 0 (`self.Material`))
  (`self.SetLifeSpan` LifeSpan)
  (set `self.isBuffActive` true))

(event `self.ReceiveBeginPlay`
  (add `PrimitiveComponent.OnComponentBeginOverlap` (`self.Sphere`) (delegate `OnComponentBeginOverlap_이벤트`)))

(event `OnComponentBeginOverlap_이벤트`
  (params (OverlappedComponent :type "PrimitiveComponent Object Reference") (OtherActor :type "Actor Object Reference") (OtherComp :type "PrimitiveComponent Object Reference") (OtherBodyIndex :type Integer) (bFromSweep :type Boolean) (SweepResult :type "HitResult Structure (by ref)"))
  (if (`self.isBuffActive`)
    (bind _asbp_xrcharacter (cast `/Game/Blueprints/Character/BP_XRCharacter` OtherActor))
    (`/Game/Blueprints/Character/BP_XRCharacter.MoveSpeedChange` _asbp_xrcharacter (`self.speedRatio`))))

(fn `UserConstructionScript`)