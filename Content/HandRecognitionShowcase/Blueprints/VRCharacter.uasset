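; VR player character for the hand recognition showcase, using pose and gesture recognizers to drive force grab and throw and to control a projector slideshow.
; An aiming pose enables the right-hand selector, a Pull gesture lerps the target to the hand, and throws launch it with amplitude-scaled impulse.
; While a head trace hits the screen, flick swipes flip slides with glowing hand cues.
; Tick also feeds recognizer results to five demo screens.
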(event `self.ReceiveBeginPlay`
  (`|ExecutionSequence`
    (:`then_0`
      (`HeadMountedDisplayFunctionLibrary.ResetOrientationAndPosition` 0.0))
    (:`then_1`
      ;[1 1 1] Interactable Selectors
      (bind _asinteractable_selector (cast `InteractableSelector` (`ChildActorComponent.ChildActor` (`self.RightSelector`))))
      (set `self.RightInteractableSelector` _asinteractable_selector))
    (:`then_2`
      ;[1 1 1] Finding the Projector Screen
      (bind _outactors (`GameplayStatics.GetAllActorsOfClass` "/Game/HandRecognitionShowcase/VRStereoProjectionScreen/VRProjectionScreen.VRProjectionScreen_C"))
      (set `self.ProjectorScreen` (`|GetArrayItem` _outactors))
      ;[1 1 1] Finding the Projector
      (bind _outactors_2 (`GameplayStatics.GetAllActorsOfClass` "/Game/HandRecognitionShowcase/VRStereoProjectionScreen/VRProjector.VRProjector_C"))
      (set `self.Projector` (`|GetArrayItem` _outactors_2)))))

(event `InputAction|LogLeftHand`
  (params (Key :type "Key Structure"))
  ;[1 1 1] Dumping hand poses and gesture state to output window
  (:`Released`
    (`HandPoseRecognizer.LogEncodedHandPose` (`self.LeftHandPoseRecognizer`))))

(event `InputAction|LogGestureState`
  (params (Key :type "Key Structure"))
  ;[1 1 1] Dumping hand poses and gesture state to output window
  (:`Released`
    (`HandGestureRecognizer.DumpAllGestureStates` (`self.RightPullPushGestureRecognizer`))))

(event `Clear Grab Candidate`
  ;[1 1 1] Selection
  (set `self.RightGrabCandidate` null))

(event `InputAction|LogRightHand`
  (params (Key :type "Key Structure"))
  ;[1 1 1] Dumping hand poses and gesture state to output window
  (:`Released`
    (`HandPoseRecognizer.LogEncodedHandPose` (`self.RightHandPoseRecognizer`))))

(event `InputAction|TogglePoseRecording`
  (params (Key :type "Key Structure"))
  ;[1 1 1] Hand Bone Range Recording
  (:`Released`
    (`/Engine/EditorBlueprintResources/StandardMacros.FlipFlop`
      (:`A`
        (`HandRecognitionFunctionLibrary.RecordHandPose` (`self.LeftHandPoseRecognizer`) :!label _label
          (:`RecordingStarted`
            (`KismetSystemLibrary.PrintString` "Recording Started" true true (struct :`R` 1.0 :`B` 0.048679 :`A` 1.0) 10.0))
          (:`RecordingStopped`
            (`KismetSystemLibrary.PrintString` "Recording Stopped" true true (struct :`R` 0.010252 :`G` 1.0 :`B` 0.015915 :`A` 1.0) 10.0))))
      (:`B`
        (goto _label :!via `StopRecording`)))))

(event `self.ReceiveTick`
  (params (DeltaSeconds :type "Float (single-precision)"))
  (bind _projectorscreen (`self.ProjectorScreen`))
  (bind _rightgrabobject (`self.RightGrabObject`))
  (bind _rightinteractableselector (`self.RightInteractableSelector`))
  (bind _rightgrabobject_2 (`self.RightGrabObject`))
  (bind _lefthandtracking (`self.LeftHandTracking`))
  (bind _projectorscreen_2 (`self.ProjectorScreen`))
  (bind _projectorscreen_3 (`self.ProjectorScreen`))
  (bind _rightgrabobject_3 (`self.RightGrabObject`))
  (bind _righthandtracking (`self.RightHandTracking`))
  (bind _rightgrabcandidate (`self.RightGrabCandidate`))
  (bind _projectorscreen_4 (`self.ProjectorScreen`))
  (bind _rightpullpushgesturerecognizer (`self.RightPullPushGestureRecognizer`))
  (bind _projectorscreen_5 (`self.ProjectorScreen`))
  (bind _rightgrabcandidate_2 (`self.RightGrabCandidate`))
  (bind _returnvalue (`PrimitiveComponent.GetMaterial` _righthandtracking 0))
  (bind _returnvalue_2 (`PrimitiveComponent.GetMaterial` _lefthandtracking 0))
  (`|ExecutionSequence`
    (:`then_0`
      (`|ExecutionSequence`
        (:`then_0`
          ;[1 1 1] Selection
          (bind (_index _name _duration) (`HandPoseRecognizer.GetRecognizedHandPose` (`self.RightPullPushPoseRecognizer`)))
          (set `self.ForcePoseName` _name)
          (if (and (`KismetStringLibrary.EqualEqual_StrStr` _name "AimingHand") (> _duration 0.1))
            (`InteractableSelector.ActivateSelector` _rightinteractableselector true)
            (bind _returnvalue_3 (`InteractableSelector.GetSelectedInteractable` _rightinteractableselector))
            (bind _output_get (set `self.RightGrabCandidate` _returnvalue_3))
            ;[1 1 1] Hover Sound
            (if (not (== (`self.PreviousRightGrabCandidate`) _output_get))
              (`/Engine/EditorBlueprintResources/StandardMacros.IsValid` _rightgrabcandidate
                (:`Is Valid`
                  (`ActorComponent.Activate` (`self.RightAudioHoverCue`) false))
                (:`Is Not Valid`
                  _))
              (set `self.PreviousRightGrabCandidate` _rightgrabcandidate))
            (else
              (`InteractableSelector.ActivateSelector` _rightinteractableselector false)
              (`KismetSystemLibrary.K2_SetTimerDelegate` (delegate `Clear Grab Candidate`) 0.1))))
        (:`then_1`
          ;[1 1 1] Force Grab
          (`/Engine/EditorBlueprintResources/StandardMacros.IsValid` (`self.RightGrabObject`)
            (:`Is Not Valid`
              (bind (_index_2 _name_2 _gesturedirection _gestureouterduration _gestureinnerduration _returnvalue_4) (`HandGestureRecognizer.GetRecognizedHandGesture` (`self.RightPullPushGestureRecognizer`) "Reset"))
              (if _returnvalue_4
                (`self.RightGestureChanged` _name_2 _gesturedirection _gestureouterduration _gestureinnerduration)
                (if (`KismetStringLibrary.EqualEqual_StrStr` _name_2 "Pull")
                  (if (`KismetSystemLibrary.IsValid` _rightgrabcandidate_2)
                    (bind _output_get_2 (set `self.RightGrabObject` _rightgrabcandidate_2))
                    (`self.SetActorCollision` (`self.RightHand`)
                      (:`  `
                        (`Interactable.SetInteractablePhysicsSimulation` _output_get_2 false)
                        (bind _output_get_3 (set `self.RightGrabObjectStart` (`self.K2_GetActorLocation` _output_get_2)))
                        ;;[1 1 1] Begin Grab Notif
                        (`Interactable.Interaction1` _rightgrabobject_2)
                        ;;[1 1 1] Force Grab Sound
                        (`ActorComponent.Activate` (`self.RightAudioForceGrab`) false)
                        (bind (_direction _alpha) (`Timeline|Teleport Timeline` :!via `PlayFromStart` :!label _label_2)
                          (:`Update`
                            (`/Engine/EditorBlueprintResources/StandardMacros.IsValid` _rightgrabobject_2
                              (:`Is Valid`
                                (`self.K2_SetActorLocation` _rightgrabobject_2 (`KismetMathLibrary.VLerp` _output_get_3 (`self.K2_GetActorLocation` (`self.RightInteractableSelector`)) _alpha) false true))
                              (:`Is Not Valid`
                                (goto _label_2 :!via `Stop`))))
                          (:`Finished`
                            (`/Engine/EditorBlueprintResources/StandardMacros.IsValid` _rightgrabobject
                              (:`Is Valid`
                                (`self.K2_AttachToActor` _rightgrabobject (`self.RightInteractableSelector`) "None" "KeepWorld" "KeepWorld" "KeepRelative" false)
                                ;;[1 1 1] Grab Complete Notif
                                (`Interactable.Interaction2` (`self.RightGrabObject`))
                                ;;[1 1 1] End of Grab Sound
                                (`ActorComponent.Deactivate` (`self.RightAudioForceGrab`))
                                (`ActorComponent.Activate` (`self.RightAudioForceGrabEnd`) true)))))))))))))
        (:`then_2`
          ;[1 1 1] Force Push
          (`/Engine/EditorBlueprintResources/StandardMacros.IsValid` (`self.RightGrabObject`)
            (:`Is Valid`
              (while (`HandGestureRecognizer.bHasRecognizedGesture` _rightpullpushgesturerecognizer)
                (bind (_index_3 _name_3 _gesturedirection_2 _gestureouterduration_2 _gestureinnerduration_2 _returnvalue_5) (`HandGestureRecognizer.GetRecognizedHandGesture` _rightpullpushgesturerecognizer "ResetAll"))
                (if _returnvalue_5
                  (bind _returnvalue_6 (`KismetMathLibrary.MultiplyMultiply_FloatFloat` (+ (/ (- (`KismetMathLibrary.FClamp` (`KismetMathLibrary.VSize` _gesturedirection_2) 20.0 40.0) 20.0) 20.0) 1.0) 2.0))
                  (`self.RightGestureChanged` _name_3 _gesturedirection_2 _gestureouterduration_2 _gestureinnerduration_2 _returnvalue_6)
                  (if (and (`KismetStringLibrary.StartsWith` _name_3 "Throw") (`KismetSystemLibrary.IsValid` _rightgrabobject_3))
                    ;;[1 1 1] Drop Notif
                    (`Interactable.Interaction3` _rightgrabobject_3)
                    (`self.K2_DetachFromActor` _rightgrabobject_3 "KeepWorld" "KeepWorld" "KeepRelative")
                    (`Interactable.SetInteractablePhysicsSimulation` _rightgrabobject_3 true)
                    (bind `_as프리미티브_컴포넌트` (cast `PrimitiveComponent` (`Actor.RootComponent` (`self.RightGrabObject`))))
                    (`PrimitiveComponent.AddImpulse` `_as프리미티브_컴포넌트` (* _gesturedirection_2 (* _returnvalue_6 20.0)) "None" false)
                    (set `self.RightGrabObject` null)
                    (`self.SetActorCollision` (`self.RightHand`) true
                      (:`  `
                        ;[1 1 1] Force Push Sound
                        (if (> _returnvalue_6 2.5)
                          (`ActorComponent.Activate` (`self.RightAudioForcePush`) false)
                          ;[1 1 1] Force Push VFX
                          (`ActorComponent.Activate` (`self.ForcePushVFX`) false))))))))))))
    (:`then_1`
      ;[1 1 1] Screen selection using swipe gestures
      (`self.IsLookingAtProjectorScreen`
        (:`Yes`
          (`/Engine/EditorBlueprintResources/StandardMacros.IsValid` _projectorscreen_3
            (:`Is Valid`
              (if (not (`self.ProjectionScreenHighlightPlayed`))
                (`/Game/HandRecognitionShowcase/VRStereoProjectionScreen/VRProjectionScreen.HighlghtScreen` _projectorscreen_3)
                (set `self.ProjectionScreenHighlightPlayed` true))
              (bind (_index_4 _name_4 _gesturedirection_3 _gestureouterduration_3 _gestureinnerduration_3 _returnvalue_7) (`HandGestureRecognizer.GetRecognizedHandGesture` (`self.RightFlickSwipeGestureRecognizer`) "ResetAll"))
              (if _returnvalue_7
                (`/Game/HandRecognitionShowcase/VRStereoProjectionScreen/VRProjectionScreen.NextScreen` _projectorscreen_4)
                ;[1 1 1] Projector Light Activates On Page Flips
                (`/Game/HandRecognitionShowcase/VRStereoProjectionScreen/VRProjector.ChangeSlide` (`self.Projector`) :!label _label_3)
                (else
                  (bind (_index_5 _name_5 _gesturedirection_4 _gestureouterduration_4 _gestureinnerduration_4 _returnvalue_8) (`HandGestureRecognizer.GetRecognizedHandGesture` (`self.LeftFlickSwipeGestureRecognizer`) "ResetAll"))
                  (if _returnvalue_8
                    (`/Game/HandRecognitionShowcase/VRStereoProjectionScreen/VRProjectionScreen.PreviousScreen` _projectorscreen_4)
                    (goto _label_3)))))))
        (:`No`
          (set `self.ProjectionScreenHighlightPlayed` false))))
    (:`then_2`
      ;[1 1 1] Slide Swipe Cues
      (`self.IsLookingAtProjectorScreen`
        (:`Yes`
          (`|ExecutionSequence`
            (:`then_0`
              (bind _returnvalue_9 (`HandGestureRecognizer.GetGestureRecognitionState` (`self.RightFlickSwipeGestureRecognizer`) 0))
              (if (`|EnumEquality` _returnvalue_9 "GestureInProgress")
                ;[1 1 1] Hand highlight cue for hand swipe gesture: lights up when gesture is started
                (bind (_direction_2 _emissiverampon) (`Timeline|Timeline_0` :!label _label_4)
                  (:`Update`
                    (`/Engine/EditorBlueprintResources/StandardMacros.IsValid` _returnvalue
                      (:`Is Valid`
                        (bind _returnvalue_10 (`PrimitiveComponent.CreateDynamicMaterialInstance` _righthandtracking 0 _returnvalue "None"))
                        (bind _output_get_4 (set `self.RightHand Material Instance` _returnvalue_10))
                        (`MaterialInstanceDynamic.SetScalarParameterValue` _output_get_4 "Emissive" _emissiverampon)))))
                (else
                  (goto _label_4 :!via `Reverse`))))
            (:`then_1`
              (bind _returnvalue_11 (`HandGestureRecognizer.GetGestureRecognitionState` (`self.LeftFlickSwipeGestureRecognizer`) 0))
              (if (`|EnumEquality` _returnvalue_11 "GestureInProgress")
                (bind (_direction_3 _emissiverampon_2) (`Timeline|Timeline_1` :!label _label_5)
                  (:`Update`
                    (`/Engine/EditorBlueprintResources/StandardMacros.IsValid` _returnvalue_2
                      (:`Is Valid`
                        (bind _returnvalue_12 (`PrimitiveComponent.CreateDynamicMaterialInstance` _lefthandtracking 0 _returnvalue_2 "None"))
                        (bind _output_get_5 (set `self.LeftHand Material Instance` _returnvalue_12))
                        (`MaterialInstanceDynamic.SetScalarParameterValue` _output_get_5 "Emissive" _emissiverampon_2)))))
                (else
                  (goto _label_5 :!via `Reverse`))))))
        (:`No`
          (`|ExecutionSequence`
            (:`then_0`
              (goto _label_4 :!via `Reverse`))
            (:`then_1`
              (goto _label_5 :!via `Reverse`))))))
    (:`then_3`
      ;[1 1 1] Screen 1: various hand poses (you can monitor a different recognizer for testing)
      (bind (_index_6 _name_6 _duration_2 _error _confidence) (`HandPoseRecognizer.GetRecognizedHandPose` (`self.LeftHandPoseRecognizer`)))
      (`/Engine/EditorBlueprintResources/StandardMacros.IsValid` _projectorscreen
        (:`Is Valid`
          (`/Game/HandRecognitionShowcase/VRStereoProjectionScreen/VRProjectionScreen.UpdateScreen1` _projectorscreen _name_6 _duration_2 _error _confidence))
        (:`Is Not Valid`
          (`/Game/HandRecognitionShowcase/VRStereoProjectionScreen/VRProjectionScreen.UpdateScreen1` _projectorscreen "None" 0.0 0.0 0.0))))
    (:`then_4`
      ;[1 1 1] Screen 2: American Sign Language Digits
      (bind (_index_7 _name_7 _duration_3 _error_2 _confidence_2) (`HandPoseRecognizer.GetRecognizedHandPose` (`self.ASLNumRecognizer`)))
      (`/Engine/EditorBlueprintResources/StandardMacros.IsValid` _projectorscreen_5
        (:`Is Valid`
          (`/Game/HandRecognitionShowcase/VRStereoProjectionScreen/VRProjectionScreen.UpdateScreen2` _projectorscreen_5 _name_7 _duration_3 _error_2 _confidence_2))
        (:`Is Not Valid`
          (`/Game/HandRecognitionShowcase/VRStereoProjectionScreen/VRProjectionScreen.UpdateScreen2` _projectorscreen_5 "None" 0.0 0.0 0.0))))
    (:`then_5`
      ;[1 1 1] Screen 3: American Sign Language Alpha (shows self occlusion issues)
      (bind (_index_8 _name_8 _duration_4 _error_3 _confidence_3) (`HandPoseRecognizer.GetRecognizedHandPose` (`self.ASLAlphaRecognizer`)))
      (`/Engine/EditorBlueprintResources/StandardMacros.IsValid` _projectorscreen_2
        (:`Is Valid`
          (`/Game/HandRecognitionShowcase/VRStereoProjectionScreen/VRProjectionScreen.UpdateScreen3` _projectorscreen_2 _name_8 _duration_4 _error_3 _confidence_3))
        (:`Is Not Valid`
          (`/Game/HandRecognitionShowcase/VRStereoProjectionScreen/VRProjectionScreen.UpdateScreen3` _projectorscreen_2 "None" 0.0 0.0 0.0))))
    (:`then_6`
      ;[1 1 1] Screen 4: Gun Gestures
      (`|ExecutionSequence`
        (:`then_0`
          (bind (_index_9 _name_9 _gesturedirection_5 _gestureouterduration_5 _gestureinnerduration_5 _returnvalue_13) (`HandGestureRecognizer.GetRecognizedHandGesture` (`self.GunGestureRecognizer`) "Reset"))
          (if _returnvalue_13
            (set `self.LastGunGesture` _name_9)))
        (:`then_1`
          (bind (_index_10 _name_10 _duration_5 _error_4 _confidence_4 _returnvalue_14) (`HandPoseRecognizer.GetRecognizedHandPose` (`self.GunPoseRecognizer`)))
          (if _returnvalue_14
            (`/Game/HandRecognitionShowcase/VRStereoProjectionScreen/VRProjectionScreen.UpdateScreen4` (`self.ProjectorScreen`) _name_10 _duration_5 _error_4 _confidence_4 (`self.LastGunGesture`))
            (else
              (`/Game/HandRecognitionShowcase/VRStereoProjectionScreen/VRProjectionScreen.UpdateScreen4` (`self.ProjectorScreen`) "None" 0.0 0.0 0.0 (`self.LastGunGesture`)))))))
    (:`then_7`
      ;[1 1 1] Screen 5: Force Grab+Push gestures (values come from swipe handling above)
      (`|ExecutionSequence`
        (:`then_0`
          (add `self.RightGestureChanged` (delegate `RightGestureChanged_Event`)))
        (:`then_1`
          (`/Game/HandRecognitionShowcase/VRStereoProjectionScreen/VRProjectionScreen.UpdateScreen5` (`self.ProjectorScreen`) (`self.ForcePoseName`) (`self.ForceGestureName`) (`self.ForceDirection`) (`self.ForceStrength`)))))))

(event `RightGestureChanged_Event` :!signature `self.RightGestureChanged`
  (params (GestureName :type String) (Direction :type "Vector Structure") (OuterDuration :type "Float (double-precision)") (InnerDuration :type "Float (double-precision)") (Force :type "Float (double-precision)"))
  ;[1 1 1] Screen 5: Force Grab+Push gestures (values come from swipe handling above)
  (set `self.ForceGestureName` GestureName)
  (set `self.ForceDirection` Direction)
  (set `self.ForceStrength` Force))

(fn `UserConstructionScript`)