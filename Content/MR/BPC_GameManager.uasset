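; Game manager Blueprint component for MR that handles Android and Quest runtime permissions at BeginPlay.
; It checks external storage write/read and Oculus scene access, adding granted entries to GrantedCount and printing success only when Add returns 2, otherwise failure.
; Each missing permission triggers a request for all three, whose callback judges success solely by the third result, scene access.
; Outcomes appear only as on-screen debug messages.
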(event `self.ReceiveBeginPlay`
  (bind _array (`|MakeArray` "android.permission.WRITE_EXTERNAL_STORAGE" "android.permission.READ_EXTERNAL_STORAGE" "com.oculus.permission.USE_SCENE"))
  (for (_array_element _array_index) _array
    (bind _returnvalue (`AndroidPermissionFunctionLibrary.CheckPermission` _array_element))
    (if _returnvalue
      (bind _returnvalue_2 (`KismetArrayLibrary.Array_Add` (`self.GrantedCount`) _array_index))
      (if (== _returnvalue_2 2)
        (`KismetSystemLibrary.PrintString` "                                                   \n \n \n \n \n \n \n \n \n                                                                                 Permission Sucess" true true (struct :`G` 0.66 :`B` 1.0 :`A` 1.0) 30.0 :!label _label)
        (else
          (`KismetSystemLibrary.PrintString` "                                                                             \n \n \n \n \n \n \n \n \n                                                                  Permission Request failed " true true (struct :`R` 1.0 :`G` 0.061523 :`A` 1.0) 30.0 :!label _label_2)))
      (else
        (bind _returnvalue_3 (`AndroidPermissionFunctionLibrary.AcquirePermissions` _array))
        (add `AndroidPermissionCallbackProxy.OnPermissionsGrantedDynamicDelegate` _returnvalue_3 (delegate `커스텀이벤트`))))))

(event `커스텀이벤트`
  (params (Permissions :type "Array of String (by ref)") (GrantResults :type "Array of Boolean (by ref)"))
  (if (`|GetArrayItem` GrantResults 2)
    (goto _label)
    (else
      (goto _label_2))))