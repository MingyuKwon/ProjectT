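; Oculus hand component that records, deletes and recognizes static hand gestures for the player.
; Gestures are named snapshots of component-space bone locations, stored in a BP_GestureSave slot and cached at BeginPlay.
; A looping timer selects the first cached gesture with every bone within a distance threshold of the live hand.
; It calls OnGestureRecognized on every poll, even without a match, as the EqualGestures change check is disconnected.
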(event `self.ReceiveBeginPlay`
  (set `self.Gestures` (`/Game/Blueprints/Player/Gesture/BP_GestureSave.Gestire` (`self.LoadGesture`)))
  (`KismetSystemLibrary.K2_SetTimerDelegate` (delegate `DetectGesture`) (`self.refreshRate`) true))

(event `DetectGesture`
  (bind (_result _gesture) (`self.GetCurrentGesture`))
  (if _result
    _
    (else
      _))
  (bind _output_get (set `self.CurrentGesture` _gesture))
  (`self.OnGestureRecognized` (`.GestureName_3_0F8A1F17443C01112E1D17A9477372D5` (break `/Game/Blueprints/Player/Gesture/Gesture` _output_get))))

(fn `DeleteGesture`
  (params (GestureName :type String))
  (locals (GestureSave :type "/Game/Blueprints/Player/Gesture/BP_GestureSave Object Reference") (index :type Integer))
  (bind _output_get (set `local.GestureSave` (`self.LoadGesture`)))
  (for (_array_element _array_index) (`/Game/Blueprints/Player/Gesture/BP_GestureSave.Gestire` _output_get)
    (if (`KismetStringLibrary.EqualEqual_StrStr` (`.GestureName_3_0F8A1F17443C01112E1D17A9477372D5` (break `/Game/Blueprints/Player/Gesture/Gesture` _array_element)) GestureName)
      (set `local.index` _array_index)))
  (`KismetArrayLibrary.Array_Remove` (`/Game/Blueprints/Player/Gesture/BP_GestureSave.Gestire` (`local.GestureSave`)) (`local.index`))
  (`GameplayStatics.SaveGameToSlot` (`local.GestureSave`) (`self.GestureSlot`)))

(fn `Does Gestire Exist`
  (params (SaveGesture :type "/Game/Blueprints/Player/Gesture/BP_GestureSave Object Reference") (GestureName :type String))
  (returns (result :type Boolean))
  (locals (NewLocalVar :type String) (L_GestureName :type String))
  (set `local.L_GestureName` GestureName)
  (for _array_element (`/Game/Blueprints/Player/Gesture/BP_GestureSave.Gestire` SaveGesture)
    (if (`KismetStringLibrary.EqualEqual_StrStr` (`.GestureName_3_0F8A1F17443C01112E1D17A9477372D5` (break `/Game/Blueprints/Player/Gesture/Gesture` _array_element)) (`local.L_GestureName`))
      (return true)))
  (return false))

(fn `EqualGestures`
  (params (A :type "/Game/Blueprints/Player/Gesture/Gesture Structure") (B :type "/Game/Blueprints/Player/Gesture/Gesture Structure"))
  (returns (NewParam :type Boolean))
  (bind (_gesturename _bonelocation) (break `/Game/Blueprints/Player/Gesture/Gesture` A))
  (bind (_gesturename_2 _bonelocation_2) (break `/Game/Blueprints/Player/Gesture/Gesture` B))
  (`KismetSystemLibrary.PrintString` _gesturename true true (struct :`R` 0.559484 :`G` 0.019449 :`B` 1.0 :`A` 1.0) -1.0 (`KismetStringLibrary.Conv_StringToName` (`KismetStringLibrary.Concat_StrStr` (`self.GestureSlot`) "a")))
  (`KismetSystemLibrary.PrintString` _gesturename_2 true true (struct :`R` 1.0 :`B` 0.074535 :`A` 1.0) -1.0 (`KismetStringLibrary.Conv_StringToName` (`KismetStringLibrary.Concat_StrStr` (`self.GestureSlot`) " d")))
  (return (and (`KismetStringLibrary.EqualEqual_StrStr` _gesturename _gesturename_2) (`KismetArrayLibrary.Array_Identical` _bonelocation _bonelocation_2))))

(fn `GetCurrentGesture`
  (returns (Result :type Boolean) (Gesture :type "/Game/Blueprints/Player/Gesture/Gesture Structure"))
  (locals (bValidGesture :type Boolean :default true) (NULLGesture :type "/Game/Blueprints/Player/Gesture/Gesture Structure" :default (struct :`GestureName` "NULL")))
  (for _array_element (`self.Gestures`)
    (for (_array_element_2 _array_index) (`.BoneLocation_7_54225610427EFF2B81FF3BA04458E21B` (break `/Game/Blueprints/Player/Gesture/Gesture` _array_element))
      (bind _returnvalue (`self.GetBoneLocationByName` (`self.GetBoneName` _array_index) "ComponentSpace"))
      (if (`self.Debug`)
        (bind _returnvalue_2 (`KismetMathLibrary.Abs` (`KismetMathLibrary.VSize` (- _returnvalue _array_element_2))))
        (`KismetSystemLibrary.PrintString` (`KismetStringLibrary.Conv_DoubleToString` _returnvalue_2) true true (struct :`G` 0.66 :`B` 1.0 :`A` 1.0) -1.0 (`KismetStringLibrary.Conv_StringToName` (`self.GestureSlot`))))
      (if (> _returnvalue_2 (`self.Threshold`))
        (set `local.bValidGesture` false)))
    (if (`local.bValidGesture`)
      (return (`local.bValidGesture`) _array_element)
      (else
        (set `local.bValidGesture` true))))
  (return false (`local.NULLGesture`)))

(fn `LoadGesture`
  (returns (SavedGesture :type "/Game/Blueprints/Player/Gesture/BP_GestureSave Object Reference"))
  (bind _returnvalue (`GameplayStatics.DoesSaveGameExist` (`self.GestureSlot`)))
  (if _returnvalue
    (bind _returnvalue_2 (`GameplayStatics.LoadGameFromSlot` (`self.GestureSlot`)))
    (bind _asbp_gesture_save (cast `/Game/Blueprints/Player/Gesture/BP_GestureSave` _returnvalue_2))
    (return _asbp_gesture_save)
    (else
      (bind _returnvalue_3 (`GameplayStatics.CreateSaveGameObject` "/Game/Blueprints/Player/Gesture/BP_GestureSave.BP_GestureSave_C"))
      (return _returnvalue_3))))

(fn `RecordGesture`
  (params (GestureName :type String))
  (locals (GestureSave :type "/Game/Blueprints/Player/Gesture/BP_GestureSave Object Reference") (BoneLocations :type "Array of Vector Structure"))
  (bind _output_get (set `local.GestureSave` (`self.LoadGesture`)))
  (bind _result (`self.Does Gestire Exist` _output_get GestureName))
  (if (not _result)
    (for _index (range (`self.GetNumBones`))
      (bind _returnvalue (`self.GetBoneLocationByName` (`self.GetBoneName` _index) "ComponentSpace"))
      (`KismetArrayLibrary.Array_Add` (`local.BoneLocations`) _returnvalue))
    (`KismetArrayLibrary.Array_Add` (`/Game/Blueprints/Player/Gesture/BP_GestureSave.Gestire` (`local.GestureSave`)) (make `/Game/Blueprints/Player/Gesture/Gesture` (`local.GestureName`) (`local.BoneLocations`)))
    (`GameplayStatics.SaveGameToSlot` (`local.GestureSave`) (`self.GestureSlot`))))