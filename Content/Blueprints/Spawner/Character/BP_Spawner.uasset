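; BP_Spawner is a one-shot placement actor that spawns an AI-controlled character at its own transform and destroys itself on BeginPlay.
; SpawnCharacter always spawns the configured SpawnClass, casts it to BP_XRCharacter and sets its on-board flag from a check of what lies beneath it.
; It then spawns a BP_XRAIController and has it possess the stored character.
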(event `self.ReceiveBeginPlay`
  (`self.Spawn Character`)
  (`self.K2_DestroyActor`))

(fn `Spawn Character`
  (locals (SpawnCHaracter :type "/Game/Blueprints/Character/BP_XRCharacter Object Reference"))
  (bind _returnvalue (`self.GetTransform`))
  (`|ExecutionSequence`
    (:`then_0`
      (bind _returnvalue_2 (`|SpawnActorFromClass` (`self.SpawnClass`) _returnvalue "AlwaysSpawn" "MultiplyWithRoot" null null))
      (bind _asbp_xrcharacter (cast `/Game/Blueprints/Character/BP_XRCharacter` _returnvalue_2))
      (bind _output_get (set `local.SpawnCHaracter` _asbp_xrcharacter))
      (bind _returnvalue_3 (`XRDefenseCharacter.CheckBeneathIsBoard` _output_get))
      (`XRDefenseCharacter.SetIsOnBoard` _output_get _returnvalue_3))
    (:`then_1`
      (bind _returnvalue_4 (`|SpawnActorFromClass` "/Game/Blueprints/AI/BP_XRAIController.BP_XRAIController_C" _returnvalue "Undefined" "MultiplyWithRoot" null null))
      (`Controller.Possess` _returnvalue_4 (`local.SpawnCHaracter`)))))

(fn `UserConstructionScript`)