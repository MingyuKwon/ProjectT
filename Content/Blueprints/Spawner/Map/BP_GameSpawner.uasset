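; BP_GameSpawner is an actor that marks where the game level is spawned when the game mode requests it.
; On BeginPlay it caches BP_ProjectTGameMode and binds a custom event to its SpawnGameLevel dispatcher.
; When triggered, it loads GameMap as a level instance at its own location and, on success, moves the found NavMeshBoundsVolume there.
; It destroys itself afterward, whether or not the load succeeded.
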(event `self.ReceiveBeginPlay`
  (`|ExecutionSequence`
    (:`then_0`
      (bind _asbp_project_tgame_mode (cast `/Game/Blueprints/GameMode/BP_ProjectTGameMode` (`GameplayStatics.GetGameMode`)))
      (set `self.As BP Project TGame Mode` _asbp_project_tgame_mode))
    (:`then_1`
      (add `/Game/Blueprints/GameMode/BP_ProjectTGameMode.SpawnGameLevel` (`self.As BP Project TGame Mode`) (delegate `커스텀이벤트`)))))

(event `커스텀이벤트`
  (`self.SpawnGame`))

(event `SpawnGame`
  (bind _boutsuccess (`LevelStreamingDynamic.LoadLevelInstance` "GameMap" (`self.K2_GetActorLocation`) (struct) "" null))
  (if _boutsuccess
    (bind _returnvalue (`GameplayStatics.GetActorOfClass` "/Script/NavigationSystem.NavMeshBoundsVolume"))
    (`self.K2_SetActorLocation` _returnvalue (`self.K2_GetActorLocation`) false false))
  (`self.K2_DestroyActor`))

(fn `UserConstructionScript`)